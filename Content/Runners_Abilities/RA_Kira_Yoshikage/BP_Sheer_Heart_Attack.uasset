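; Sheer Heart Attack, a ground-following projectile actor for the Kira Yoshikage runner's ability.
; A timeline drives it along world X by a speed-scaled step, applying hand-rolled gravity whenever a downward trace finds no ground.
; Every tick AttackAbilityComponent traces from the Cube for damage; a hit destroys the actor, adding a voice line after a short delay.
; If the timeline finishes first, it spawns an explosion and destroys itself.
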(event EventBeginPlay
  (bind _returnvalue (Transformation|GetActorLocation))
  (Utilities|FlowControl|Sequence
    (:then_0
      (Audio|PlaySound2D "/Game/Sounds/SFX/Abilities/RA_Kira/Siege_Trebuchet_Fire_Shot.Siege_Trebuchet_Fire_Shot" 1.0 1.0 0.0 0 0))
    (:then_1
      (Timeline|SHA_Timeline PlayFromStart
        (:Update
          (Utilities|FlowControl|Sequence
            (:then_0
              (bind (_outhit _returnvalue_2) (Collision|LineTraceByChannel (+ _returnvalue "0,0.000000,100.000000") (+ _returnvalue "0, 0,-50.000000") "TraceTypeQuery1" false 0 "None"))
              (if _returnvalue_2
                (Variables|Default|SetG 0.0)
                (else
                  (Transformation|AddActorWorldOffset (Math|Vector|MakeVector 0.0 0.0 (Variables|Default|GetG)))
                  (Variables|Default|SetG (+ (Variables|Default|GetG) -9.8)))))
            (:then_1
              (Transformation|AddActorWorldOffset (Math|Vector|MakeVector (* 1.1e+02 (Variables|Default|GetSpeed_Multiplier)) 0.0 0.0)))))
        (:Finished
          (Game|SpawnActorfromClass "/Game/Effects/FX_Explosion01.FX_Explosion01_C" (Transformation|GetActorTransform) "Undefined" 0 true "0.000000,0.000000,0.000000|0.000000,0.000000,0.000000|1.000000,1.000000,1.000000" 10 "/Game/World/Chunk_Types/Asphalt_Mat.Asphalt_Mat" 0)
          (Actor|DestroyActor))
        (:Voice
          (Audio|PlaySound2D "/Game/Sounds/Voice/Kira/Ability_01.Ability_01" 1.0 1.0 0.0 0 0))))))

(event EventTick
  (params (DeltaSeconds :type Float%20%28single-precision%29))
  (Variables|Default|SetTimer (+ DeltaSeconds (Variables|Default|GetTimer)))
  (bind _returnvalue (Default|AttackTraceFunction (Variables|Default|GetAttack_Ability_Component) (Variables|Default|GetCube) 1e+03 1e+02 "NewEnumerator0" false "0, 0, 0" "None" (Utilities|Array|MakeArray self)))
  (if _returnvalue
    (Utilities|FlowControl|Sequence
      (:then_0
        (Actor|DestroyActor))
      (:then_1
        (if (>= (Variables|Default|GetTimer) 1.1)
          (Audio|PlaySound2D "/Game/Sounds/Voice/Kira/Ability_02.Ability_02" 1.0 1.0 0.0 0 0))))))

(fn ConstructionScript)